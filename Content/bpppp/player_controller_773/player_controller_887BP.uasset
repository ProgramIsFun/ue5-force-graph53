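; Player controller Blueprint that sets up a Graphcontrol4 UI panel and lets the player switch to operating it with the mouse.
; On BeginPlay it creates the widget, adds it to the viewport and keeps a reference to it.
; Pressing 1 prints a debug string, shows the cursor and sets UI-only input.
; Nodes for hiding the cursor and restoring game-only input are unconnected, so this Blueprint never switches back.
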(event EventBeginPlay
  (bind _returnvalue (UserInterface|CreateWidget "/Game/bpppp/UI7/WIDGET8/graphcontrol4.graphcontrol4_C" (Game|GetPlayerController 0)))
  (UserInterface|Viewport|AddtoViewport _returnvalue 19)
  (Variables|Default|Setgraph_control_panel_738 _returnvalue))

(event EventTick
  (params (DeltaSeconds :type Float%20%28single-precision%29)))

(event Input|KeyboardEvents|1
  (params (Key :type Key%20Structure :default "None"))
  (bind _returnvalue (Game|GetPlayerController 0))
  (:Pressed
    (Development|PrintString "Hello")
    (Variables|/Script/Engine.PlayerController|SetbShowMouseCursor _returnvalue true)
    (Input|SetInputModeUIOnly _returnvalue 0 "DoNotLock" false)))

(fn ConstructionScript)