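; BP_A is a spline-based spawner actor that repeatedly creates BP_B actors at the spline's first point.
; On BeginPlay it caches the world locations of spline points 0 and 1, then starts a looping timer at SpawnTime intervals.
; Each tick of that timer spawns a BP_B, passing it both endpoints and Speed.
; The construction script spaces Num collision-free static meshes evenly along the spline with a fixed relative rotation.
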(event Custom|Move
  (bind _beginlocation (Variables|Default|GetBeginLocation))
  (Game|SpawnActorfromClass "/Game/TRASH777/BP_B.BP_B_C" (Math|Transform|MakeTransform _beginlocation "0, 0, 0" "1.000000,1.000000,1.000000") "AlwaysSpawn" "MultiplyWithRoot" 0 (Variables|Default|GetEndLocation) _beginlocation (Variables|Default|GetSpeed) 0))

(event Custom|Go
  (bind _returnvalue (Utilities|Time|SetTimerbyEvent (delegate Custom|Move) (Variables|Default|GetSpawnTime) true))
  (Variables|Default|SetTimer _returnvalue))

(event EventBeginPlay
  (Variables|Default|SetBeginLocation (Spline|GetLocationatSplinePoint (Variables|Default|GetSpline) 0 "World"))
  (Variables|Default|SetEndLocation (Spline|GetLocationatSplinePoint (Variables|Default|GetSpline) 1 "World"))
  (CallFunction|Go))

(fn ConstructionScript
  (bind _num (Variables|Default|GetNum))
  (if (> _num 0)
    (for _index (range 0 (- _num 1))
      (bind _returnvalue (AddComponent|AddStaticMeshComponent false (Math|Transform|MakeTransform (Math|Transform|TransformLocation (Math|Transform|InvertTransform (Transformation|GetActorTransform)) (Spline|GetLocationatDistanceAlongSpline (Variables|Default|GetSpline) (Math|Conversions|ToFloat(Integer) (* _index (/ (Spline|GetSplineLength (Variables|Default|GetSpline)) (- _num 1)))) "World")))))
      (Transformation|SetRelativeRotation _returnvalue "-90.000000,0.000000,0.000000" false false)
      (Collision|SetCollisionEnabled _returnvalue "NoCollision"))))